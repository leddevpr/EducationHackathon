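; A clickable piano Blueprint with seven keys, Do through Si, for a note-matching game on a musical staff.
; Clicking a key plays its 2D sound and stores its note number, one to seven, in NotaPiano.
; It then fetches the pentagram actor from the GM game mode and calls its Match function with that number.
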(event OnClicked(Do)
  (params (TouchedComponent :type Primitive%20Component%20Object%20Reference) (ButtonPressed :type Key%20Structure))
  (Audio|PlaySound2D "/Game/SonidosNotas/Do.Do" 1.0 1.0 0.0 0 0)
  (Variables|Default|SetnotaPiano 1)
  (CallFunction|Match))

(event OnClicked(Re)
  (params (TouchedComponent :type Primitive%20Component%20Object%20Reference) (ButtonPressed :type Key%20Structure))
  (Audio|PlaySound2D "/Game/SonidosNotas/Re.Re" 1.0 1.0 0.0 0 0)
  (Variables|Default|SetnotaPiano 2)
  (CallFunction|Match))

(event OnClicked(Mi)
  (params (TouchedComponent :type Primitive%20Component%20Object%20Reference) (ButtonPressed :type Key%20Structure))
  (Audio|PlaySound2D "/Game/SonidosNotas/Mi.Mi" 1.0 1.0 0.0 0 0)
  (Variables|Default|SetnotaPiano 3)
  (CallFunction|Match))

(event OnClicked(Fa)
  (params (TouchedComponent :type Primitive%20Component%20Object%20Reference) (ButtonPressed :type Key%20Structure))
  (Audio|PlaySound2D "/Game/SonidosNotas/Fa.Fa" 1.0 1.0 0.0 0 0)
  (Variables|Default|SetnotaPiano 4)
  (CallFunction|Match))

(event OnClicked(Sol)
  (params (TouchedComponent :type Primitive%20Component%20Object%20Reference) (ButtonPressed :type Key%20Structure))
  (Audio|PlaySound2D "/Game/SonidosNotas/Sol.Sol" 1.0 1.0 0.0 0 0)
  (Variables|Default|SetnotaPiano 5)
  (CallFunction|Match))

(event OnClicked(La)
  (params (TouchedComponent :type Primitive%20Component%20Object%20Reference) (ButtonPressed :type Key%20Structure))
  (Audio|PlaySound2D "/Game/SonidosNotas/La.La" 1.0 1.0 0.0 0 0)
  (Variables|Default|SetnotaPiano 6)
  (CallFunction|Match))

(event OnClicked(Si)
  (params (TouchedComponent :type Primitive%20Component%20Object%20Reference) (ButtonPressed :type Key%20Structure))
  (Audio|PlaySound2D "/Game/SonidosNotas/Si.Si" 1.0 1.0 0.0 0 0)
  (Variables|Default|SetnotaPiano 7)
  (CallFunction|Match))

(event Custom|match
  (bind _asgm (Utilities|Casting|CastToGM (Game|GetGameMode)))
  (bind _aspentagramabp (Utilities|Casting|CastTopentagramabp (Variables|/Game/GM.GM_C|Getpentagrama _asgm)))
  (Default|Match _aspentagramabp (Variables|Default|GetnotaPiano)))

(event EventBeginPlay)

(fn ConstructionScript)