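; Musical staff actor for a timed note-recognition game that registers itself with the GM game mode.
; It spawns a RedondaBP note at a random staff position, avoiding immediate repeats, and plays its pitch through a sound cue parameter.
; Match compares piano input to that note, shows feedback, scores hits and spawns the next.
; A looping one-second timer drives the countdown display, then reports the score to GM and opens an end widget.
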(event Custom|note%20spawn
  (if (not (Variables|Default|GetendGame?))
    (bind _output_get (Variables|Default|SetrandNum (Math|Random|RandomInteger 8)))
    (if (!= (Variables|Default|GetspawnNum) _output_get)
      (bind _output_get_2 (Variables|Default|SetspawnNum _output_get))
      (switch int _output_get_2
        (:0
          (Variables|Default|Setlocation (Transformation|GetWorldTransform (Variables|Default|GetSpawn)))
          (Variables|Default|Setnotapuesta 3))
        (:1
          (Variables|Default|Setlocation (Transformation|GetWorldTransform (Variables|Default|Getspawn2)))
          (Variables|Default|Setnotapuesta 4))
        (:2
          (Variables|Default|Setlocation (Transformation|GetWorldTransform (Variables|Default|Getspawn3)))
          (Variables|Default|Setnotapuesta 5))
        (:3
          (Variables|Default|Setlocation (Transformation|GetWorldTransform (Variables|Default|Getspawn4)))
          (Variables|Default|Setnotapuesta 6))
        (:4
          (Variables|Default|Setlocation (Transformation|GetWorldTransform (Variables|Default|Getspawn5)))
          (Variables|Default|Setnotapuesta 7))
        (:5
          (Variables|Default|Setlocation (Transformation|GetWorldTransform (Variables|Default|Getspawn6)))
          (Variables|Default|Setnotapuesta 1))
        (:6
          (Variables|Default|Setlocation (Transformation|GetWorldTransform (Variables|Default|Getspawn7)))
          (Variables|Default|Setnotapuesta 2))
        (:7
          (Variables|Default|Setlocation (Transformation|GetWorldTransform (Variables|Default|Getspawn8)))
          (Variables|Default|Setnotapuesta 3))
        (:8
          (Variables|Default|Setlocation (Transformation|GetWorldTransform (Variables|Default|Getspawn9)))
          (Variables|Default|Setnotapuesta 3)))
      (bind _returnvalue (Game|SpawnActorfromClass "/Game/redondaBP.redondaBP_C" (Variables|Default|Getlocation) "Undefined" 0 0))
      (Variables|Default|Setnota _returnvalue)
      (CallFunction|PlaySound)
      (else
        (CallFunction|NoteSpawn)))))

(event Custom|match
  (params (notaPiano :type Integer))
  (bind _good_job (Variables|Default|GetGood%20Job))
  (bind _sorry_try_again (Variables|Default|GetSorry%20Try%20Again))
  (if (== notaPiano (Variables|Default|Getnotapuesta))
    (Rendering|SetVisibility _good_job true false)
    (bind _output_get (Variables|Default|SetscoreVar (+ (Variables|Default|GetscoreVar) 1)))
    (Rendering|Components|TextRender|SetText (Variables|Default|GetscoreNum) (Utilities|Text|ToText(Integer) _output_get))
    (Utilities|FlowControl|Delay 0.5)
    (Rendering|SetVisibility _good_job false false)
    (Actor|DestroyActor (Variables|Default|Getnota))
    (CallFunction|NoteSpawn)
    (else
      (Rendering|SetVisibility _sorry_try_again true false)
      (Utilities|FlowControl|Delay 2.0)
      (Rendering|SetVisibility _sorry_try_again false false)
      (Actor|DestroyActor (Variables|Default|Getnota))
      (CallFunction|NoteSpawn))))

(event Custom|PlaySound
  (bind _notacue (Variables|Default|GetnotaCue))
  (Effects|Components|ParticleSystem|SetIntParameter _notacue "nota" (Variables|Default|Getnotapuesta))
  (Audio|Components|Audio|Play _notacue 0.0))

(event Custom|timer
  (Utilities|FlowControl|Sequence
    (:then_0
      (Variables|Default|SetSeconds (- (Variables|Default|GetSeconds) 1))
      (if (< (Variables|Default|GetSeconds) 0)
        (Variables|Default|SetSeconds 9)
        (Variables|Default|SetSeconds2 (- (Variables|Default|GetSeconds2) 1))
        (if (< (Variables|Default|GetSeconds2) 0)
          (Variables|Default|SetMinutes (- (Variables|Default|GetMinutes) 1))
          (Variables|Default|SetSeconds2 5)
          (Variables|Default|SetSeconds 9)
          (if (< (Variables|Default|GetMinutes) 0)
            (Variables|Default|SetMinutes 0)
            (Variables|Default|SetSeconds2 0)
            (Variables|Default|SetSeconds 0)
            (Utilities|FlowControl|DoOnce false
              (:Completed
                (Utilities|Time|ClearandInvalidateTimerbyHandle (Variables|Default|Gettimer1))
                (Variables|Default|SetendGame? true)
                (bind _asgm (Utilities|Casting|CastToGM (Game|GetGameMode)))
                (Default|EndGame _asgm (Variables|Default|GetscoreVar))
                (Variables|Default|SetMinutes 1)
                (bind _returnvalue (UserInterface|CreateWidget "/Game/ui.ui_C"))
                (UserInterface|Viewport|AddtoViewport _returnvalue 0)))))))
    (:then_1
      (Rendering|Components|TextRender|SetText (Variables|Default|GetSegundos) (Utilities|Text|ToText(Integer) (Variables|Default|GetSeconds)))
      (Rendering|Components|TextRender|SetText (Variables|Default|GetSegundos2) (Utilities|Text|ToText(Integer) (Variables|Default|GetSeconds2)))
      (Rendering|Components|TextRender|SetText (Variables|Default|GetMinutos) (Utilities|Text|ToText(Integer) (Variables|Default|GetMinutes))))))

(event Custom|startGames
  (CallFunction|NoteSpawn)
  (bind _returnvalue (Utilities|Time|SetTimerbyEvent (delegate Custom|timer) 1.0 true))
  (Variables|Default|Settimer1 _returnvalue))

(event EventBeginPlay
  (bind _asgm (Utilities|Casting|CastToGM (Game|GetGameMode)))
  (Variables|/Game/GM.GM_C|Setpentagrama _asgm self))

(fn ConstructionScript)